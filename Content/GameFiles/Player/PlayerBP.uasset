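; Player character for a mouse-aimed shooter, with axis movement, sprint, gunfire and health.
; Tick yaws the capsule toward the cursor hit point, and firing spawns a bullet at a reference component unless the anim blueprint reports sprinting.
; BeginPlay shows the cursor plus kill count and health widgets.
; Damage plays sounds and random montages; at zero health it disables movement and calls GameLose on the game mode.
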(event `InputAction|Fire`
  (params (Key :type "Key Structure"))
  (bind _bullet_ref (`self.Bullet REF`))
  ;[1 1 1] Fire Gun
  (:`Pressed`
    (bind _asue4asp_hero_tpp_anim_blueprint (cast `/Game/GameFiles/Player/UE4ASP_HeroTPP_AnimBlueprint` (`SkeletalMeshComponent.GetAnimInstance` (`self.Mesh`))))
    (if (not (`/Game/GameFiles/Player/UE4ASP_HeroTPP_AnimBlueprint.IsSprinting` _asue4asp_hero_tpp_anim_blueprint))
      (`|SpawnActorFromClass` "/Game/GameFiles/Guns/BulletBP.BulletBP_C" (`KismetMathLibrary.MakeTransform` (`SceneComponent.K2_GetComponentLocation` _bullet_ref) (`KismetMathLibrary.MakeRotFromZ` (`SceneComponent.GetForwardVector` _bullet_ref)) (0.4 0.4 0.4)) "Undefined" "OverrideRootScale" null null))))

(event `InputAxis|MoveForward`
  (params (AxisValue :type "Float (single-precision)"))
  ;[1 1 1] Basic Movement
  (`self.AddMovementInput` (`KismetMathLibrary.GetForwardVector` (`KismetMathLibrary.MakeRotator` 0.0 0.0 (.yaw (`self.GetControlRotation`)))) AxisValue))

(event `self.ReceiveTick`
  (params (DeltaSeconds :type "Float (single-precision)"))
  (bind (_returnvalue_roll _returnvalue_pitch) (`KismetMathLibrary.BreakRotator` (`self.K2_GetActorRotation`)))
  (bind (_returnvalue_roll_2 _returnvalue_pitch_2 _returnvalue_yaw) (`KismetMathLibrary.BreakRotator` (`KismetMathLibrary.FindLookAtRotation` (`self.K2_GetActorLocation`) (`.Location` (`GameplayStatics.BreakHitResult` (`PlayerController.GetHitResultUnderCursorByChannel` (`GameplayStatics.GetPlayerController` 0) "TraceTypeQuery1" true))))))
  ;[1 1 1] Make Player Face Mouse
  (if (not (`self.IsDead?`))
    (`SceneComponent.K2_SetWorldRotation` (`self.CapsuleComponent`) (`KismetMathLibrary.MakeRotator` _returnvalue_roll _returnvalue_pitch _returnvalue_yaw) false false)))

(event `InputAxis|MoveRight`
  (params (AxisValue :type "Float (single-precision)"))
  ;[1 1 1] Basic Movement
  (`self.AddMovementInput` (`KismetMathLibrary.GetRightVector` (`KismetMathLibrary.MakeRotator` 0.0 0.0 (.yaw (`self.GetControlRotation`)))) AxisValue))

(event `self.ReceiveBeginPlay`
  (bind _returnvalue (`GameplayStatics.GetPlayerController` 0))
  ;[1 1 1] Enable Mouse During Gameplay
  (set `PlayerController.bShowMouseCursor` true _returnvalue)
  (`Controller.SetIgnoreMoveInput` _returnvalue false)
  (bind _returnvalue_2 (`|CreateWidget` "/Game/GameFiles/UI/KillCountWidget.KillCountWidget_C"))
  (`UserWidget.AddToViewport` _returnvalue_2 0)
  (bind _returnvalue_3 (`|CreateWidget` "/Game/GameFiles/UI/HealthWidget.HealthWidget_C"))
  (`UserWidget.AddToViewport` _returnvalue_3 0))

(event `InputAction|Sprint`
  (params (Key :type "Key Structure"))
  (bind _charactermovement (`self.CharacterMovement`))
  ;[1 1 1] Sprint
  (:`Pressed`
    (set `CharacterMovementComponent.MaxWalkSpeed` 450.0 _charactermovement))
  (:`Released`
    (set `CharacterMovementComponent.MaxWalkSpeed` 175.0 _charactermovement)))

(event `self.ReceiveAnyDamage`
  (params (Damage :type "Float (single-precision)") (DamageType :type "DamageType Object Reference") (InstigatedBy :type "Controller Object Reference") (DamageCauser :type "Actor Object Reference"))
  (bind _returnvalue (`self.K2_GetActorLocation`))
  (if (not (`self.IsDead?`))
    (bind _output_get (set `self.Health` (`KismetMathLibrary.FClamp` (- (`self.Health`) Damage) 0.0 100.0)))
    (if (== _output_get 0.0)
      (`GameplayStatics.PlaySoundAtLocation` null _returnvalue (struct) 1.0 1.0 0.0 null null null)
      (`CharacterMovementComponent.DisableMovement` (`self.CharacterMovement`))
      (set `self.IsDead?` true)
      (`self.PlayAnimMontage` (select `int` (`KismetMathLibrary.RandomInteger` 1) :`0` null :`1` null :!type "AnimMontage Object Reference") 2.0)
      (bind _asmain_game_mode (cast `/Game/GameFiles/Blueprints/MainGameMode` (`GameplayStatics.GetGameMode`)))
      (`/Game/GameFiles/Blueprints/MainGameMode.Game Lose` _asmain_game_mode)
      (else
        (`GameplayStatics.PlaySoundAtLocation` null _returnvalue (struct) 1.0 1.0 0.0 null null null)
        (bind _returnvalue_2 (`self.PlayAnimMontage` (select `int` (`KismetMathLibrary.RandomInteger` 3) :`0` null :`1` null :`2` null :`3` null :!type "AnimMontage Object Reference") 2.0))
        (`KismetSystemLibrary.Delay` _returnvalue_2)))))

(fn `UserConstructionScript`)