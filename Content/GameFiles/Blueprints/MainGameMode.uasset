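; MainGameMode is the game mode that tracks the enemy population and runs a five-minute kill-goal match with win and lose screens.
; Events adjust the alive-enemy count, and BeginPlay triggers a single delayed increase of the enemy cap alongside the match timer.
; A self-rescheduling event refreshes the countdown widget every second.
; Timer expiry shows game over if kills fall short, while GameWin has no caller here.
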(event `Increase Enemies`
  (`/Engine/EditorBlueprintResources/StandardMacros.IncrementInt` (`self.Enemies Alive`)))

(event `Decrease Enemies`
  (`/Engine/EditorBlueprintResources/StandardMacros.DecrementInt` (`self.Enemies Alive`)))

(event `Increase Limit`
  (params (Duration :type "Float (double-precision)") (`Increase Amount` :type "Float (double-precision)"))
  (`KismetSystemLibrary.Delay` Duration)
  (set `self.Max Enemies` (`KismetMathLibrary.FTrunc` (* (`self.Max Enemies`) `Increase Amount`))))

(event `self.ReceiveBeginPlay`
  (`|ExecutionSequence`
    (:`then_0`
      (`self.Increase Limit` 10.0 1.1))
    (:`then_1`
      (`self.Game Timer`))))

(event `Game Lose`
  (bind _asplayer_bp (cast `/Game/GameFiles/Player/PlayerBP` (`GameplayStatics.GetPlayerCharacter` 0)))
  (if (not (>= (`/Game/GameFiles/Player/PlayerBP.Kills` _asplayer_bp) (`self.KillGoal`)))
    (`self.DisableInput` (`GameplayStatics.GetPlayerPawn` 0) null)
    (bind _returnvalue (`|CreateWidget` "/Game/GameFiles/UI/GameOverScreen.GameOverScreen_C"))
    (`UserWidget.AddToViewport` _returnvalue 0)))

(event `Game Timer`
  (bind _returnvalue (`KismetSystemLibrary.K2_SetTimerDelegate` (delegate `Game Lose`) 300.0))
  (bind _returnvalue_2 (`|CreateWidget` "/Game/GameFiles/UI/TimerWidget.TimerWidget_C"))
  (bind _output_get (set `self.Timer REF` _returnvalue_2))
  (`UserWidget.AddToViewport` _output_get 0)
  (`self.Update Time`))

(event `Update Time`
  (`KismetSystemLibrary.K2_SetTimerDelegate` (delegate `Update Time`) 1.0)
  (set `/Game/GameFiles/UI/TimerWidget.Time Remaining` (`KismetSystemLibrary.K2_GetTimerRemainingTimeHandle` (stale `Game Timer` _returnvalue)) (`self.Timer REF`)))

(event `Game Win`
  (`self.DisableInput` (`GameplayStatics.GetPlayerPawn` 0) null)
  (bind _returnvalue (`|CreateWidget` "/Game/GameFiles/UI/WinScreen.WinScreen_C"))
  (`UserWidget.AddToViewport` _returnvalue 0))

(fn `UserConstructionScript`)