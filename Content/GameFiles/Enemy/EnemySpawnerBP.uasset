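; Enemy spawner actor that keeps spawning batches of a configurable enemy class at its own transform while MainGameMode is under its enemy limit.
; BeginPlay spawns the first batch unconditionally and caches the game mode.
; After each SpawnDelay, EnemiesAlive is compared to MaxEnemies, either spawning another full batch or polling again through ShouldSpawn.
; The endless loop uses self-calling events with Delays rather than Tick or timers.
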(event `self.ReceiveBeginPlay`
  (`|ExecutionSequence`
    (:`then_0`
      (`self.Spawn Enemy` (`self.Enemy`) (`self.GetTransform`) (`self.Number Of Enemies`)))
    (:`then_1`
      (bind _asmain_game_mode (cast `/Game/GameFiles/Blueprints/MainGameMode` (`GameplayStatics.GetGameMode`)))
      (set `self.Game Mode REF` _asmain_game_mode))))

(event `Spawn Enemy`
  (params (Enemy :type "Actor Class Reference") (SpawnTransform :type "Transform Structure") (`Number Of Enemies` :type Integer))
  (bind _game_mode_ref (`self.Game Mode REF`))
  (for _ (range `Number Of Enemies`)
    (`|SpawnActorFromClass` Enemy SpawnTransform "Undefined" "OverrideRootScale" null null))
  (`KismetSystemLibrary.Delay` (`self.Spawn Delay`))
  (if (< (`/Game/GameFiles/Blueprints/MainGameMode.Enemies Alive` _game_mode_ref) (`/Game/GameFiles/Blueprints/MainGameMode.Max Enemies` _game_mode_ref))
    (`self.Spawn Enemy` (`self.Enemy`) (`self.GetTransform`) (`self.Number Of Enemies`))
    (else
      (`self.ShouldSpawn?`))))

(event `ShouldSpawn?`
  (bind _game_mode_ref (`self.Game Mode REF`))
  (`KismetSystemLibrary.Delay` (`self.Spawn Delay`))
  (if (< (`/Game/GameFiles/Blueprints/MainGameMode.Enemies Alive` _game_mode_ref) (`/Game/GameFiles/Blueprints/MainGameMode.Max Enemies` _game_mode_ref))
    (`self.Spawn Enemy` (`self.Enemy`) (`self.GetTransform`) (`self.Number Of Enemies`))
    (else
      (`self.ShouldSpawn?`))))

(fn `UserConstructionScript`)