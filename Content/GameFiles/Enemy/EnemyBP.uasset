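; Gun-wielding enemy character that chases the player and fires bullets until killed.
; BeginPlay randomises walk speed, registers with MainGameMode and starts two self-repeating loops: AI move-to with turn-to-face, and shooting at random intervals.
; Non-lethal damage pauses movement for a random hit montage.
; Death plays a montage, credits the player's kill, updates MainGameMode's counts, triggers the win at the kill goal, and destroys the actor afterwards.
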(event `Chase Player`
  (params (`Player To Chase` :type "/Game/GameFiles/Player/PlayerBP Object Reference"))
  (bind (_returnvalue_roll _returnvalue_pitch) (`KismetMathLibrary.BreakRotator` (`self.K2_GetActorRotation`)))
  (bind (_returnvalue_roll_2 _returnvalue_pitch_2 _returnvalue_yaw) (`KismetMathLibrary.BreakRotator` (`KismetMathLibrary.FindLookAtRotation` (`self.K2_GetActorLocation`) (`CharacterMovementComponent.GetLastUpdateLocation` (`Character.CharacterMovement` (`GameplayStatics.GetPlayerCharacter` 0))))))
  ;[1 1 1] Chase Player
  (if (not (`self.IsDead?`))
    (bind _asplayer_bp (cast `/Game/GameFiles/Player/PlayerBP` (`GameplayStatics.GetPlayerCharacter` 0)))
    (if (`/Game/GameFiles/Player/PlayerBP.IsDead?` _asplayer_bp)
      (`CharacterMovementComponent.DisableMovement` (`self.CharacterMovement`))
      (else
        (`|AIMoveTo` self (0.0 0.0 0.0) `Player To Chase` 250.0
          (:`OnSuccess`
            _)
          (:`OnFail`
            _))
        (`SceneComponent.K2_SetWorldRotation` (`self.CapsuleComponent`) (`KismetMathLibrary.MakeRotator` _returnvalue_roll _returnvalue_pitch _returnvalue_yaw) false false)
        (`self.Chase Player` (`self.Char REF`))))))

(event `Shoot Player`
  (bind _bullet_ref (`self.Bullet REF`))
  (bind _returnvalue (`SceneComponent.K2_GetComponentLocation` _bullet_ref))
  ;[1 1 1] Fire Gun
  (if (not (`self.IsDead?`))
    (`|SpawnActorFromClass` "/Game/GameFiles/Guns/EnemyBulletBP.EnemyBulletBP_C" (`KismetMathLibrary.MakeTransform` _returnvalue (`KismetMathLibrary.MakeRotFromZ` (`SceneComponent.GetForwardVector` _bullet_ref)) (0.2 0.2 0.2)) "Undefined" "OverrideRootScale" null null :!label _label)
    (`GameplayStatics.PlaySoundAtLocation` null _returnvalue (struct) 1.0 1.0 0.0 null null null)
    (`GameplayStatics.SpawnEmitterAttached` null (`self.FX REF`) "None" (0.0 0.0 0.0) (struct :`Yaw` 90.0) (6.0 6.0 6.0))
    (`KismetSystemLibrary.Delay` (select `int` (`KismetMathLibrary.RandomInteger` 3) :`0` 1.5 :`1` 2.0 :`2` 2.5 :`3` 3.0 :!type "Float (single-precision)"))
    (`self.Shoot Player`)))

(event `self.ReceiveBeginPlay`
  (`|ExecutionSequence`
    (:`then_0`
      ;[1 1 1] Spawn Enemies & Set Speeds
      (bind _asplayer_bp (cast `/Game/GameFiles/Player/PlayerBP` (`GameplayStatics.GetPlayerCharacter` 0)))
      (bind _output_get (set `self.Char REF` _asplayer_bp))
      (`self.Chase Player` _output_get)
      (set `CharacterMovementComponent.MaxWalkSpeed` (select `int` (`KismetMathLibrary.RandomInteger` 3) :`0` 100.0 :`1` 125.0 :`2` 150.0 :`3` 170.0 :!type "Float (single-precision)") (`self.CharacterMovement`))
      (bind _asmain_game_mode (cast `/Game/GameFiles/Blueprints/MainGameMode` (`GameplayStatics.GetGameMode`)))
      (`/Game/GameFiles/Blueprints/MainGameMode.Increase Enemies` _asmain_game_mode))
    (:`then_1`
      (goto _label))))

(event `self.ReceiveAnyDamage`
  (params (Damage :type "Float (single-precision)") (DamageType :type "DamageType Object Reference") (InstigatedBy :type "Controller Object Reference") (DamageCauser :type "Actor Object Reference"))
  (bind _returnvalue (`self.K2_GetActorLocation`))
  (if (not (`self.IsDead?`))
    (bind _output_get (set `self.Health` (`KismetMathLibrary.FClamp` (- (`self.Health`) Damage) 0.0 100.0)))
    (if (== _output_get 0.0)
      (`GameplayStatics.PlaySoundAtLocation` null _returnvalue (struct) 1.0 1.0 0.0 null null null)
      (`CharacterMovementComponent.DisableMovement` (`self.CharacterMovement`))
      (set `self.IsDead?` true)
      (`PrimitiveComponent.SetCollisionEnabled` (`self.Mesh`) "NoCollision")
      (bind _returnvalue_2 (`self.PlayAnimMontage` (select `int` (`KismetMathLibrary.RandomInteger` 1) :`0` null :`1` null :!type "AnimMontage Object Reference") 2.0))
      (`|ExecutionSequence`
        (:`then_0`
          (bind _asplayer_bp (cast `/Game/GameFiles/Player/PlayerBP` (`GameplayStatics.GetPlayerCharacter` 0)))
          (if (not (`/Game/GameFiles/Player/PlayerBP.IsDead?` _asplayer_bp))
            (`/Engine/EditorBlueprintResources/StandardMacros.IncrementInt` (`/Game/GameFiles/Player/PlayerBP.Kills` _asplayer_bp))))
        (:`then_1`
          (`KismetSystemLibrary.Delay` _returnvalue_2)
          (`self.K2_DestroyActor`)
          (bind _asmain_game_mode (cast `/Game/GameFiles/Blueprints/MainGameMode` (`GameplayStatics.GetGameMode`)))
          (`/Game/GameFiles/Blueprints/MainGameMode.Decrease Enemies` _asmain_game_mode))
        (:`then_2`
          (bind _asmain_game_mode_2 (cast `/Game/GameFiles/Blueprints/MainGameMode` (`GameplayStatics.GetGameMode`)))
          (set `/Game/GameFiles/Blueprints/MainGameMode.Enemies Killed` (+ (`/Game/GameFiles/Blueprints/MainGameMode.Enemies Killed` _asmain_game_mode_2) 1) _asmain_game_mode_2))
        (:`then_3`
          (bind _asmain_game_mode_3 (cast `/Game/GameFiles/Blueprints/MainGameMode` (`GameplayStatics.GetGameMode`)))
          (if (>= (`/Game/GameFiles/Blueprints/MainGameMode.Enemies Killed` _asmain_game_mode_3) (`/Game/GameFiles/Blueprints/MainGameMode.KillGoal` _asmain_game_mode_3))
            (bind _asmain_game_mode_4 (cast `/Game/GameFiles/Blueprints/MainGameMode` (`GameplayStatics.GetGameMode`)))
            (`/Game/GameFiles/Blueprints/MainGameMode.Game Win` _asmain_game_mode_4))))
      (else
        (`GameplayStatics.PlaySoundAtLocation` null _returnvalue (struct) 1.0 1.0 0.0 null null null)
        (`CharacterMovementComponent.DisableMovement` (`self.CharacterMovement`))
        (bind _returnvalue_3 (`self.PlayAnimMontage` (select `int` (`KismetMathLibrary.RandomInteger` 3) :`0` null :`1` null :`2` null :`3` null :!type "AnimMontage Object Reference") 2.0))
        (`KismetSystemLibrary.Delay` _returnvalue_3)
        (if (not (`self.IsDead?`))
          (`CharacterMovementComponent.SetMovementMode` (`self.CharacterMovement`) "MOVE_Walking" 0))))))

(fn `UserConstructionScript`)