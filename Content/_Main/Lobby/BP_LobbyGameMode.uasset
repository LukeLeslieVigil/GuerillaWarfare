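; BP_LobbyGameMode is the game mode for the multiplayer lobby, setting up each player who joins.
; On PostLogin it records the player, caches PlayerStart actors and reads server name and max players from the Steam game instance.
; It then initializes the player controller's lobby menu and default map settings through reference messages.
; It finally calls SpawnPlayer, whose event body is still empty.
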(event `self.K2_PostLogin`
  (params (NewPlayer :type "PlayerController Object Reference"))
  (bind _output_get (set `self.ConnectedPlayer` NewPlayer))
  (`KismetArrayLibrary.Array_AddUnique` (`self.Players`) _output_get)
  (bind _outactors (`GameplayStatics.GetAllActorsOfClass` "/Script/Engine.PlayerStart"))
  (set `self.SpawnPoints` _outactors)
  (bind _gameinstance (message `/Game/_Main/BPI_GameInstance.SteamGameInstanceRef` (`GameplayStatics.GetGameInstance`)))
  (set `self.ServerName` (`/Game/_Main/GuerillaGameInstance.ServerName` _gameinstance))
  (set `self.MaxPlayers` (`/Game/_Main/GuerillaGameInstance.MaxPlayers` _gameinstance))
  (bind _lobbypc (message `/Game/_Main/Lobby/BPI_LobbyPC.LobbyPCRef` (`self.ConnectedPlayer`)))
  (`/Game/_Main/Lobby/Guerilla_Lobby_PC.InitialSetup` _lobbypc)
  (`/Game/_Main/Lobby/Guerilla_Lobby_PC.SetupLobbyMenu` _lobbypc (`self.ServerName`))
  (`/Game/_Main/Lobby/Guerilla_Lobby_PC.UpdateLobbySettings` _lobbypc (`self.DefaultMapImage`) (`self.DefaultMapName`) (`self.DefaultMapTime`))
  (`self.SpawnPlayer` (`self.ConnectedPlayer`)))

(event `SpawnPlayer`
  (params (Player :type "PlayerController Object Reference")))

(fn `UserConstructionScript`)